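; Game mode for a UI-driven Trump–Kim negotiation game, swapping side-select, game, lost-trust and end screens.
; StartGame stores the chosen allegiance, and NextRound adds each leader's trade and military values to running totals.
; A player lead beyond the military, trade or combined threshold earns a strike, with three losing trust.
; Otherwise demands reset each meeting until the fifth, when CheckEndResults picks the EndState from the player's relative standing.
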(event Custom|StartGame
  (params (Allegiance :type Enum_Allegiance%20Enum :default "NewEnumerator0"))
  (bind _returnvalue (Game|GetPlayerController 0))
  (Variables|Default|SetCurrentAllegiance Allegiance)
  (Widget|RemovefromParent (Variables|Default|GetCurrentWidget))
  (bind _returnvalue_2 (UserInterface|CreateWidget "/Game/Blueprints/GameWBP.GameWBP_C"))
  (Variables|Default|SetCurrentWidget _returnvalue_2)
  (UserInterface|Viewport|AddtoViewport _returnvalue_2 0)
  (Input|SetInputModeUIOnly _returnvalue _returnvalue_2 "DoNotLock")
  (Variables|/Script/Engine.PlayerController|SetbShowMouseCursor _returnvalue true))

(event Custom|NextRound
  (params (TrumpTradeValue :type Integer) (TrumpMilitaryValue :type Integer) (KimTradeValue :type Integer) (KimMilitaryValue :type Integer))
  (bind _meetingnumber (Variables|Default|GetMeetingNumber))
  ;[1 1 1] Adds Value at End of Round
  (Utilities|FlowControl|Sequence
    (:then_0
      (Variables|Default|SetTrumpTradeValue (+ TrumpTradeValue (Variables|Default|GetTrumpTradeValue))))
    (:then_1
      (Variables|Default|SetTrumpMilitaryValue (+ TrumpMilitaryValue (Variables|Default|GetTrumpMilitaryValue))))
    (:then_2
      (Variables|Default|SetKimTradeValue (+ KimTradeValue (Variables|Default|GetKimTradeValue))))
    (:then_3
      (Variables|Default|SetKimMilitaryValue (+ KimMilitaryValue (Variables|Default|GetKimMilitaryValue))))
    (:then_4
      (Utilities|FlowControl|Sequence
        (:then_0
          ;[1 1 1] Checks if enemy loosing trust
          (if (> (Math|Integer|Absolute(Integer) (- (Variables|Default|GetTrumpMilitaryValue) (Variables|Default|GetKimMilitaryValue))) 5)
            (switch Utilities|FlowControl|Switch|SwitchonEnum_Allegiance (Variables|Default|GetCurrentAllegiance)
              (:NewEnumerator1
                (if (< (Variables|Default|GetKimMilitaryValue) (Variables|Default|GetTrumpMilitaryValue))
                  (bind _result (Math|Integer|IncrementInt (Variables|Default|GetStrikes) :!label _label)
                    (:%20%20
                      (Development|PrintString (Utilities|String|ToString(Integer) _result))))))
              (:NewEnumerator2
                (if (not (< (Variables|Default|GetKimMilitaryValue) (Variables|Default|GetTrumpMilitaryValue)))
                  (goto _label))))
            (elif (> (Math|Integer|Absolute(Integer) (- (Variables|Default|GetTrumpTradeValue) (Variables|Default|GetKimTradeValue))) 8)
              (switch Utilities|FlowControl|Switch|SwitchonEnum_Allegiance (Variables|Default|GetCurrentAllegiance)
                (:NewEnumerator1
                  (if (< (Variables|Default|GetKimTradeValue) (Variables|Default|GetTrumpTradeValue))
                    (goto _label)))
                (:NewEnumerator2
                  (if (not (< (Variables|Default|GetKimTradeValue) (Variables|Default|GetTrumpTradeValue)))
                    (goto _label))))
              (elif (> (Math|Integer|Absolute(Integer) (- (+ (Variables|Default|GetTrumpTradeValue) (Variables|Default|GetTrumpMilitaryValue)) (+ (Variables|Default|GetKimTradeValue) (Variables|Default|GetKimMilitaryValue)))) 10)
                (switch Utilities|FlowControl|Switch|SwitchonEnum_Allegiance (Variables|Default|GetCurrentAllegiance)
                  (:NewEnumerator1
                    (if (< (+ (Variables|Default|GetKimMilitaryValue) (Variables|Default|GetKimTradeValue)) (+ (Variables|Default|GetTrumpMilitaryValue) (Variables|Default|GetTrumpTradeValue)))
                      (goto _label)))
                  (:NewEnumerator2
                    (if (not (< (+ (Variables|Default|GetKimMilitaryValue) (Variables|Default|GetKimTradeValue)) (+ (Variables|Default|GetTrumpMilitaryValue) (Variables|Default|GetTrumpTradeValue))))
                      (goto _label))))))))
        (:then_3
          ;[1 1 1] Switches to different states if conditions are met
          (if (== (Variables|Default|GetStrikes) 3)
            (Widget|RemovefromParent (Variables|Default|GetCurrentWidget))
            (bind _returnvalue (UserInterface|CreateWidget "/Game/Blueprints/WBP_LostTrust.WBP_LostTrust_C"))
            (Variables|Default|SetCurrentWidget _returnvalue)
            (UserInterface|Viewport|AddtoViewport _returnvalue 0)
            (elif (== _meetingnumber 5)
              (CallFunction|CheckEndResults)
              (Widget|RemovefromParent (Variables|Default|GetCurrentWidget))
              (bind _returnvalue_2 (UserInterface|CreateWidget "/Game/Blueprints/WBP_EndGame.WBP_EndGame_C"))
              (Variables|Default|SetCurrentWidget _returnvalue_2)
              (UserInterface|Viewport|AddtoViewport _returnvalue_2 0)
              (else
                (Math|Integer|IncrementInt _meetingnumber
                  (:%20%20
                    (bind _asgame_wbp (Utilities|Casting|CastToGameWBP (Variables|Default|GetCurrentWidget)))
                    (Default|ResetDemands _asgame_wbp)
                    (Variables|Default|SetSelectedIcons 0)))))))))))

(event Custom|CheckEndResults
  (bind _trumptradevalue (Variables|Default|GetTrumpTradeValue))
  (bind _trumpmilitaryvalue (Variables|Default|GetTrumpMilitaryValue))
  (bind _kimtradevalue (Variables|Default|GetKimTradeValue))
  (bind _kimmilitaryvalue (Variables|Default|GetKimMilitaryValue))
  (bind _trumpmilitaryvalue_2 (Variables|Default|GetTrumpMilitaryValue))
  (bind _kimmilitaryvalue_2 (Variables|Default|GetKimMilitaryValue))
  (bind _kimtradevalue_2 (Variables|Default|GetKimTradeValue))
  (bind _trumptradevalue_2 (Variables|Default|GetTrumpTradeValue))
  (bind _trumpmilitaryvalue_3 (Variables|Default|GetTrumpMilitaryValue))
  (bind _kimmilitaryvalue_3 (Variables|Default|GetKimMilitaryValue))
  (bind _kimtradevalue_3 (Variables|Default|GetKimTradeValue))
  (bind _trumptradevalue_3 (Variables|Default|GetTrumpTradeValue))
  (bind _returnvalue (+ _kimtradevalue _kimmilitaryvalue))
  (bind _returnvalue_2 (+ _trumpmilitaryvalue _trumptradevalue))
  ;[1 1 1] Checks if Allegiance is strong enough
  (switch Utilities|FlowControl|Switch|SwitchonEnum_Allegiance (Variables|Default|GetCurrentAllegiance)
    (:NewEnumerator1
      (if (> _returnvalue _returnvalue_2)
        (Variables|Default|SetEndState "NewEnumerator1")
        (elif (< _trumpmilitaryvalue_3 _kimmilitaryvalue_3)
          (if (> (Math|Integer|Absolute(Integer) (- _trumpmilitaryvalue_3 _kimmilitaryvalue_3)) 5)
            (Variables|Default|SetEndState "NewEnumerator2")
            (else
              (if (< _trumptradevalue_3 _kimtradevalue_3) :!label _label
                (if (> (Math|Integer|Absolute(Integer) (- _trumptradevalue_3 _kimtradevalue_3)) 8)
                  (Variables|Default|SetEndState "NewEnumerator3")
                  (else
                    (Variables|Default|SetEndState "NewEnumerator0" :!label _label_2)))
                (else
                  (goto _label_2)))))
          (else
            (goto _label)))))
    (:NewEnumerator2
      (if (> _returnvalue_2 _returnvalue)
        (Variables|Default|SetEndState "NewEnumerator1")
        (elif (< _kimmilitaryvalue_2 _trumpmilitaryvalue_2)
          (if (> (Math|Integer|Absolute(Integer) (- _kimmilitaryvalue_2 _trumpmilitaryvalue_2)) 5)
            (Variables|Default|SetEndState "NewEnumerator2")
            (else
              (if (< _kimtradevalue_2 _trumptradevalue_2) :!label _label_3
                (if (> (Math|Integer|Absolute(Integer) (- _kimtradevalue_2 _trumptradevalue_2)) 8)
                  (Variables|Default|SetEndState "NewEnumerator3")
                  (else
                    (Variables|Default|SetEndState "NewEnumerator0" :!label _label_4)))
                (else
                  (goto _label_4)))))
          (else
            (goto _label_3)))))))

(event EventBeginPlay
  (bind _returnvalue (Game|GetPlayerController 0))
  (bind _returnvalue_2 (UserInterface|CreateWidget "/Game/Blueprints/WBP_SideSelect.WBP_SideSelect_C"))
  (Variables|Default|SetCurrentWidget _returnvalue_2)
  (UserInterface|Viewport|AddtoViewport _returnvalue_2 0)
  (Input|SetInputModeUIOnly _returnvalue _returnvalue_2 "DoNotLock")
  (Variables|/Script/Engine.PlayerController|SetbShowMouseCursor _returnvalue true))

(event EventTick
  (params (DeltaSeconds :type Float%20%28single-precision%29)))

(fn ConstructionScript)